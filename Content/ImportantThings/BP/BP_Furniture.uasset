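; BP_Furniture is a furniture actor that takes its mesh from the PC actor's PCMesh on spawn and reveals it after a short delay.
; Clicking it shows a plane and sets a Rotate flag, letting Left and Right keys turn the mesh in 90-degree yaw steps.
; Releasing the click hides the plane and disables input, ending rotation.
; Overlapping a BP_Wall sets a Colliding flag, which is never cleared here.
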(event EventBeginPlay
  (Input|EnableInput (Game|GetPlayerController 0))
  (bind _returnvalue (Actor|GetActorOfClass "/Game/ImportantThings/System/PC.PC_C"))
  (Variables|Default|SetPC _returnvalue)
  (Components|StaticMesh|SetStaticMesh (Variables|Default|GetStaticMesh) (Variables|/Game/ImportantThings/System/PC.PC_C|GetPCMesh _returnvalue))
  (Utilities|FlowControl|Delay 0.15)
  (Utilities|IsValid self
    (:Is%20Valid
      (Rendering|SetVisibility (Variables|Default|GetStaticMesh) true false))))

(event MouseInput|EventActorOnClicked
  (params (ButtonPressed :type Key%20Structure :default "None"))
  (if (not (Variables|Default|GetRotate))
    (Rendering|SetVisibility (Variables|Default|GetPlane) true false)
    (Variables|Default|SetRotate true)))

(event EventActorOnReleased
  (params (ButtonReleased :type Key%20Structure :default "None"))
  (Rendering|SetVisibility (Variables|Default|GetPlane) false false)
  (Input|DisableInput (Game|GetPlayerController 0)))

(event Collision|EventActorBeginOverlap
  (params (OtherActor :type Actor%20Object%20Reference))
  (Utilities|Casting|CastToBP_Wall OtherActor)
  (Variables|Default|SetColliding true))

(event Input|KeyboardEvents|Right
  (params (Key :type Key%20Structure :default "None"))
  (bind _staticmesh (Variables|Default|GetStaticMesh))
  (:Pressed
    (if (Variables|Default|GetRotate)
      (Transformation|SetRelativeRotation _staticmesh (Math|Rotator|MakeRotator 0.0 0.0 (+ (.yaw (Variables|/Script/Engine.SceneComponent|GetRelativeRotation _staticmesh)) 9e+01)) false false))))

(event Input|KeyboardEvents|Left
  (params (Key :type Key%20Structure :default "None"))
  (bind _staticmesh (Variables|Default|GetStaticMesh))
  (:Pressed
    (if (Variables|Default|GetRotate)
      (Transformation|SetRelativeRotation _staticmesh (Math|Rotator|MakeRotator 0.0 0.0 (- (.yaw (Variables|/Script/Engine.SceneComponent|GetRelativeRotation _staticmesh)) 9e+01)) false false))))

(fn ConstructionScript)