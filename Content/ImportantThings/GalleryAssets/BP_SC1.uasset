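; BP_SC1 is an actor that snaps to the player's current camera viewpoint and saves that transform when key 1 is pressed.
; On BeginPlay it enables input from the first player controller and caches a PC actor reference.
; The key press copies the PlayerCameraManager transform to itself and into a new SG_All save object, written to the "Transform" slot.
; Nothing here loads the saved transform back.
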(event EventBeginPlay
  (Input|EnableInput (Game|GetPlayerController 0))
  (bind _returnvalue (Actor|GetActorOfClass "/Game/ImportantThings/System/PC.PC_C"))
  (Variables|Default|SetPC _returnvalue))

(event Input|KeyboardEvents|1
  (params (Key :type Key%20Structure))
  (:Pressed
    (bind _returnvalue (Actor|GetActorOfClass "/Script/Engine.PlayerCameraManager"))
    (Transformation|SetActorTransform (Transformation|GetActorTransform _returnvalue))
    (bind _returnvalue_2 (SaveGame|CreateSaveGameObject "/Game/ImportantThings/System/SG_All.SG_All_C"))
    (Variables|/Game/ImportantThings/System/SG_All.SG_All_C|SetTransform1 _returnvalue_2 (Transformation|GetActorTransform _returnvalue))
    (SaveGame|SaveGametoSlot _returnvalue_2 "Transform")))

(fn ConstructionScript)